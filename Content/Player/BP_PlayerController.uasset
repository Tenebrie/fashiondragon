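; BP_PlayerController is a player controller that provides two debug events.
; OnShowAnimDebug toggles the WBP_Anim_00_Debug widget, creating it and adding it to the viewport, or removing it and clearing the stored DebugMenu reference.
; OnDebugButton2 casts the game mode to MainGameMode and calls RestartGame on it.
; BeginPlay, Tick and the construction script are empty.
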(event EventBeginPlay)

(event EventTick
  (params (DeltaSeconds :type Float%20%28single-precision%29)))

(event EventOnShowAnimDebug
  (if (Utilities|IsValid (Variables|Default|GetDebugMenu))
    (Widget|RemovefromParent (Variables|Default|GetDebugMenu))
    (Variables|Default|SetDebugMenu 0)
    (else
      (bind _returnvalue (UserInterface|CreateWidget "/Game/UI/WBP_Anim_00_Debug.WBP_Anim_00_Debug_C"))
      (bind _output_get (Variables|Default|SetDebugMenu _returnvalue))
      (UserInterface|Viewport|AddtoViewport _output_get 0))))

(event EventOnDebugButton2
  (bind _asmain_game_mode (Utilities|Casting|CastToMainGameMode (Game|GetGameMode)))
  (Class|GameMode|RestartGame _asmain_game_mode))

(fn ConstructionScript)